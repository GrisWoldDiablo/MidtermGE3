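; BP_Bear is a shootable bear that flashes when hit and is destroyed when its HP runs out.
; Overlaps with FirstPersonProjectile actors decrement HP, then either set Lerp to full or destroy the bear at zero or below.
; BeginPlay creates a dynamic material instance on the Bear component, and Tick fades its Lerp parameter back to zero over one second.
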(event `self.ReceiveBeginPlay`
  (bind _returnvalue (`PrimitiveComponent.CreateDynamicMaterialInstance` (`self.Bear`) 0 null "None"))
  (set `self.Material` _returnvalue))

(event `self.ReceiveTick`
  (params (DeltaSeconds :type "Float (single-precision)"))
  (bind _output_get (set `self.Lerp` (`KismetMathLibrary.FClamp` (- (`self.Lerp`) DeltaSeconds))))
  (`MaterialInstanceDynamic.SetScalarParameterValue` (`self.Material`) "Lerp" _output_get))

(event `self.ReceiveActorBeginOverlap`
  (params (OtherActor :type "Actor Object Reference"))
  (bind _hp (`self.HP`))
  (cast `/Game/FirstPersonBP/Blueprints/FirstPersonProjectile` OtherActor)
  (`/Engine/EditorBlueprintResources/StandardMacros.DecrementInt` _hp
    (:`  `
      (`/Engine/EditorBlueprintResources/StandardMacros.CompareInt` _hp
        (:`>`
          (bind _output_get (set `self.Lerp` 1.0))
          (`MaterialInstanceDynamic.SetScalarParameterValue` (`self.Material`) "Lerp" _output_get))
        (:`==`
          (`self.K2_DestroyActor` :!label _label))
        (:`<`
          (goto _label))))))

(fn `UserConstructionScript`)