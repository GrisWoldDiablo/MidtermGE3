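; BP_Client is a client actor that the player serves by hitting it with a projectile.
; On overlap with a FirstPersonProjectile, it destroys the projectile and flips its Twist flag, which nothing in this graph reads.
; The first such hit also marks the client as Served and increments the served count on the player's FirstPersonCharacter, so each client counts once.
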(event `self.ReceiveActorBeginOverlap`
  (params (OtherActor :type "Actor Object Reference"))
  (bind _asfirst_person_projectile (cast `/Game/FirstPersonBP/Blueprints/FirstPersonProjectile` OtherActor))
  (`self.K2_DestroyActor` _asfirst_person_projectile)
  (set `self.Twist` (not (`self.Twist`)))
  (if (not (`self.Served`))
    (set `self.Served` true)
    (bind _asfirst_person_character (cast `/Game/FirstPersonBP/Blueprints/FirstPersonCharacter` (`GameplayStatics.GetPlayerCharacter` 0)))
    (`/Engine/EditorBlueprintResources/StandardMacros.IncrementInt` (`/Game/FirstPersonBP/Blueprints/FirstPersonCharacter.Served Quatity` _asfirst_person_character))))

(fn `UserConstructionScript`)